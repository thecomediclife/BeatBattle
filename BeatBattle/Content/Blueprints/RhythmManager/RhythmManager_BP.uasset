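; Rhythm manager that plays the selected BGM track, tracks its beats from the BPM and judges player beat inputs.
; Audio playback percent drives the current time, auto-completing a beat as a miss once its post-tolerance window passes.
; Inputs inside the pre/post tolerance window complete the beat and send the player controller a success message, otherwise a fail.
; Each completed beat fires a dispatch and advances the counter, resyncing it to playback time when it lags.
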(event `self.ReceiveBeginPlay`
  (bind _audio (`self.Audio`))
  (bind (_output_soundcue _output_bpm) (break `/Game/Blueprints/RhythmManager/GameplayBGM_Struct` (`|GetArrayItem` (`self.Gameplay_BGM_Data`) (`self.Selectedsong`))))
  (bind _output_soundcue_2 (break `/Game/Blueprints/RhythmManager/GameplayBGM_Struct` (`|GetArrayItem` (`self.Gameplay_BGM_Data`) (`self.Selectedsong`))))
  (`AudioComponent.SetSound` (`self.Audio`) _output_soundcue_2)
  (add `AudioComponent.OnAudioPlaybackPercent` _audio (delegate `AudioPlaybackPercent`))
  (set `self.BeatCounter` 0)
  (set `self.TimePerBeat` (/ 1.0 (/ (`KismetMathLibrary.Conv_IntToDouble` _output_bpm) 60.0)))
  (`AudioComponent.Play` _audio 0.0)
  (`self.MusicBegan_Dispatch`))

(event `AudioPlaybackPercent`
  (params (PlayingSoundWave :type "SoundWave Object Reference") (PlaybackPercent :type "Float (double-precision)"))
  (bind _duration (`SoundBase.Duration` (`AudioComponent.Sound` (`self.Audio`))))
  (bind _returnvalue (* PlaybackPercent _duration))
  (set `self.CurrentPlaybackTime` _returnvalue)
  (`KismetSystemLibrary.PrintString` (`KismetStringLibrary.Conv_DoubleToString` _returnvalue) false true (struct :`G` 0.66 :`B` 1.0 :`A` 1.0) (`GameplayStatics.GetWorldDeltaSeconds`))
  (if (>= (* PlaybackPercent _duration) (+ (* (+ (`self.BeatCounter`) 1) (`self.TimePerBeat`)) (* (`self.PostBeatTolerance`) (`self.TimePerBeat`))))
    (`self.BeatComplete_Dispatch`)
    (`self.IncrementBeatCounterAndAutoCorrect`)
    (`KismetSystemLibrary.PrintString` "MISS!!!" true true (struct :`G` 0.010046 :`B` 1.0 :`A` 1.0))))

(event `InputtedBeat`
  (bind _timeperbeat (`self.TimePerBeat`))
  (bind _returnvalue (* (+ (`self.BeatCounter`) 1) (`self.TimePerBeat`)))
  (if (and (!= (`self.LastInputtedBeat`) (`self.BeatCounter`)) (`KismetMathLibrary.InRange_FloatFloat` (`self.CurrentPlaybackTime`) (- _returnvalue (* (`self.PreBeatTolerance`) (`self.TimePerBeat`))) (+ _returnvalue (* (`self.PostBeatTolerance`) (`self.TimePerBeat`)))))
    (`self.BeatComplete_Dispatch`)
    (`self.IncrementBeatCounterAndAutoCorrect`)
    (message `/Game/Blueprints/Interfaces/ReceiveBeat_Interface.BeatSuccess` (`GameplayStatics.GetPlayerController` 0))
    (`KismetSystemLibrary.PrintString` "Success" true true (struct :`G` 0.66 :`B` 1.0 :`A` 1.0) _timeperbeat)
    (set `self.LastPlaybackTime` (`self.CurrentPlaybackTime`))
    (else
      (message `/Game/Blueprints/Interfaces/ReceiveBeat_Interface.BeatFail` (`GameplayStatics.GetPlayerController` 0))
      (`KismetSystemLibrary.PrintString` "MISS!!!" true true (struct :`R` 1.0 :`G` 0.008526 :`A` 1.0) _timeperbeat))))

(fn `CalculateTimePerBeat`
  (bind (_output_soundcue _output_bpm) (break `/Game/Blueprints/RhythmManager/GameplayBGM_Struct` (`|GetArrayItem` (`self.Gameplay_BGM_Data`) (`self.Selectedsong`))))
  (set `self.TimePerBeat` (/ 1.0 (/ (`KismetMathLibrary.Conv_IntToDouble` _output_bpm) 60.0))))

(fn `IncrementBeatCounterAndAutoCorrect`
  (bind _returnvalue (`KismetMathLibrary.FFloor` (/ (`self.CurrentPlaybackTime`) (`self.TimePerBeat`))))
  (`|ExecutionSequence`
    (:`then_0`
      (if (< (`self.BeatCounter`) (- _returnvalue 1))
        (set `self.BeatCounter` _returnvalue)))
    (:`then_1`
      (set `self.LastInputtedBeat` (`self.BeatCounter`))
      (`/Engine/EditorBlueprintResources/StandardMacros.IncrementInt` (`self.BeatCounter`)))))

(fn `UserConstructionScript`)