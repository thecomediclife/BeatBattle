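; Test player pawn that defines its own movement and two attacks.
; Move offsets the actor without sweep, scaling the input offset by a move multiplier and the game state's grid size.
; Attack1 spawns a TestPlayer_Attack1_BP actor at the shooting start point.
; Attack2 fires a debug-drawn Visibility trace along world +Y and sends DamagedMessage to the hit actor.
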(event `self.Move`
  (params (WorldOffset :type "Vector Structure"))
  ;[1 1 1] How this pawn moves
  (`self.K2_AddActorWorldOffset` (* WorldOffset (* (`self.MoveMultiplier`) (`/Game/GameMode/BeatBattle_GameState_BP.GridSize` (`self.GameStateRef`))))))

(event `self.Attack1`
  ;[1 1 1] How this pawn attacks
  (`|SpawnActorFromClass` "/Game/Blueprints/Player/TestPlayer/TestPlayer_Attack1_BP.TestPlayer_Attack1_BP_C" (`KismetMathLibrary.MakeTransform` (`SceneComponent.K2_GetComponentLocation` (`self.ShootingStartLocation`))) "Undefined" "OverrideRootScale" null 25.0 null))

(event `self.Attack2`
  (bind _returnvalue (`self.K2_GetActorLocation`))
  ;[1 1 1] How this pawn attacks
  (bind _outhit (`KismetSystemLibrary.LineTraceSingle` :`Start` _returnvalue :`End` (+ _returnvalue (0.0 1000.0 0.0)) :`TraceChannel` "TraceTypeQuery1" :`DrawDebugType` "ForDuration" :`DrawTime` 1.0))
  (message `/Game/Blueprints/Interfaces/Damageable_Interface.Damaged` (`.HitActor` (`GameplayStatics.BreakHitResult` _outhit)) 10.0))

(fn `UserConstructionScript`
  (`parent.UserConstructionScript`))