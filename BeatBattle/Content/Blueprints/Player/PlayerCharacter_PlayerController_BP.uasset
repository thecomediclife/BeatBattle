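; Player controller for the Beat Battle game that only lets the pawn move or attack when input lands on the beat.
; BeginPlay retries every 0.2 seconds for the game state's RhythmManager, then sets the level's Camera_BP as view target and caches the pawn.
; Each input reports to the RhythmManager, then calls the pawn's action only if the success flag, set by the manager's BeatSuccess and BeatFail events, is true.
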(event `self.ReceiveBeginPlay`
  ;[1 1 1] Get RhythmManager Reference
  (bind _asbeat_battle_game_state_bp (cast `/Game/GameMode/BeatBattle_GameState_BP` (`GameplayStatics.GetGameState`) :!label _label)
    (:`then`
      (bind _rhythmmanagerref (`/Game/GameMode/BeatBattle_GameState_BP.RhythmManagerRef` _asbeat_battle_game_state_bp)
        (:`then`
          (set `self.RhythmManagerRef` _rhythmmanagerref))
        (:`else`
          (`KismetSystemLibrary.Delay` 0.2)
          (goto _label))))
    (:`CastFailed`
      _))
  ;[1 1 1] Set Camera actor and set it to view target
  (bind _outactors (`GameplayStatics.GetAllActorsOfClass` "/Game/Blueprints/Player/Camera_BP.Camera_BP_C"))
  (bind _output_get (set `self.CameraRef` (`|GetArrayItem` _outactors)))
  (`self.SetViewTargetWithBlend` _output_get)
  ;[1 1 1] Save Player Pawn Reference
  (bind _asplayer_character_pawn_bp (cast `/Game/Blueprints/Player/PlayerCharacter_Pawn_BP` (`GameplayStatics.GetPlayerPawn` 0)))
  (set `self.PlayerRef` _asplayer_character_pawn_bp))

(event `InputAction|Move_Up`
  (params (Key :type "Key Structure"))
  ;[1 1 1] Player Pawn Movement
  (:`Pressed`
    (`self.InputBeat`)
    (`self.AttemptToMove` (1.0 0.0 0.0))))

(event `InputAction|Attack_1`
  (params (Key :type "Key Structure"))
  ;[1 1 1] Player Pawn Attack 1 and 2
  (:`Pressed`
    (`self.InputBeat`)
    (`self.AttemptToAttack1`)))

(event `InputAction|Move_Left`
  (params (Key :type "Key Structure"))
  ;[1 1 1] Player Pawn Movement
  (:`Pressed`
    (`self.InputBeat`)
    (`self.AttemptToMove` (0.0 -1.0 0.0))))

(event `InputAction|Attack_2`
  (params (Key :type "Key Structure"))
  ;[1 1 1] Player Pawn Attack 1 and 2
  (:`Pressed`
    (`self.InputBeat`)
    (`self.AttemptToAttack2`)))

(event `InputAction|Move_Down`
  (params (Key :type "Key Structure"))
  ;[1 1 1] Player Pawn Movement
  (:`Pressed`
    (`self.InputBeat`)
    (`self.AttemptToMove` (-1.0 0.0 0.0))))

(event `InputAction|Move_Right`
  (params (Key :type "Key Structure"))
  ;[1 1 1] Player Pawn Movement
  (:`Pressed`
    (`self.InputBeat`)
    (`self.AttemptToMove` (0.0 1.0 0.0))))

(event `/Game/Blueprints/Interfaces/ReceiveBeat_Interface.BeatSuccess`
  ;[1 1 1] Message received from RhythmManager_BP whether beat is succesful or not
  (set `self.BeatSuccess?` true))

(event `/Game/Blueprints/Interfaces/ReceiveBeat_Interface.BeatFail`
  ;[1 1 1] Message received from RhythmManager_BP whether beat is succesful or not
  (set `self.BeatSuccess?` false))

(fn `AttemptToAttack1`
  (if (`self.BeatSuccess?`)
    (`/Game/Blueprints/Player/PlayerCharacter_Pawn_BP.Attack1` (`self.PlayerRef`))))

(fn `AttemptToAttack2`
  (if (`self.BeatSuccess?`)
    (`/Game/Blueprints/Player/PlayerCharacter_Pawn_BP.Attack2` (`self.PlayerRef`))))

(fn `AttemptToMove`
  (params (DeltaLocation :type "Vector Structure"))
  (if (`self.BeatSuccess?`)
    (`/Game/Blueprints/Player/PlayerCharacter_Pawn_BP.Move` (`self.PlayerRef`) DeltaLocation)))

(fn `InputBeat`
  (`/Game/Blueprints/RhythmManager/RhythmManager_BP.InputtedBeat` (`self.RhythmManagerRef`)))

(fn `UserConstructionScript`)